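; BasicEnemy is an enemy Blueprint with attack, chase and kill behavior.
; Attack briefly swaps the Body material as a visual cue, then broadcasts OnAttackEnd; no damage is applied here.
; ChasePlayer uses AIMoveTo toward the player character when IsSeeiingPlayer is true, but OnSeePawn is empty and the logic setting that flag is disconnected.
; KillEnemy simply destroys the actor.
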(event `Attack`
  (bind _body (`self.Body`))
  (`PrimitiveComponent.SetMaterial` _body 0 "/Game/BlueTransparen.BlueTransparen")
  (`KismetSystemLibrary.Delay` 0.2)
  (`PrimitiveComponent.SetMaterial` _body 0 "/Game/Imported_Models/Buildings/Door.Door")
  (`self.OnAttackEnd`))

(event `self.PawnSensing.OnSeePawn`
  (params (Pawn :type "Pawn Object Reference")))

(event `Chase Player`
  (if (`self.IsSeeiingPlayer`)
    (`AITask_MoveTo.AIMoveTo` (`AIBlueprintHelperLibrary.GetAIController` self) (0.0 0.0 0.0) (`GameplayStatics.GetPlayerCharacter` 0))))

(fn `KillEnemy`
  (`self.K2_DestroyActor`))

(fn `UserConstructionScript`)