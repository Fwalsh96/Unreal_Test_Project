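; Basic enemy character Blueprint that exposes melee attack, patrol route and movement speed functions.
; MeleeAttack briefly swaps the mesh material as a visual cue, then calls OnAttackEnd.
; GetPatrolRoute returns the stored route, and SetMovementSpeed maps idle, walking and sprinting states to the character's max walk speed.
; BeginPlay and ChasePlayer are empty, leaving the montage playback and move-to-player nodes disconnected.
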(event `Melee Attack`
  (bind _mesh (`self.Mesh`))
  (`PrimitiveComponent.SetMaterial` _mesh 0 "/Game/BlueTransparen.BlueTransparen")
  (`KismetSystemLibrary.Delay` 0.2)
  (`PrimitiveComponent.SetMaterial` _mesh 0 "/Game/Imported_Models/Buildings/Door.Door")
  (`self.OnAttackEnd`))

(event `self.ReceiveBeginPlay`)

(event `Chase Player`)

(fn `GetPatrolRoute`
  (returns (`Patrol Route` :type "/Game/AI/PatrolRoute Object Reference"))
  (return (`self.PatrolRoute`)))

(fn `SetMovementSpeed`
  (params (Speed :type "/Game/AI/Enums/E_EnemySpeed Enum" :default "NewEnumerator0"))
  (returns (SpeedValue :type "Float (double-precision)"))
  (bind _output_get (set `CharacterMovementComponent.MaxWalkSpeed` (select `/Game/AI/Enums/E_EnemySpeed` Speed :`NewEnumerator1` 100.0 :`NewEnumerator2` 500.0 :!type "Float (single-precision)") (`self.CharacterMovement`)))
  (return _output_get))

(fn `UserConstructionScript`)