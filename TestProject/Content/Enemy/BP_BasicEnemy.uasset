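; Basic enemy that chases the first player from BeginPlay, re-issuing AIMoveTo 0.2 seconds after each success, with no retry on failure.
; It also carries player-style functions, none called from the event graph: weapon swapping, magazine and reserve ammo, and health and armor.
; These read the first player's controller and push values to NewHUD.
; Kill and armor-break only log, IsInteractable returns false, and IsInteractionObservable is empty.
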(event `self.ReceiveBeginPlay`
  (`self.Chase Player`))

(event `Chase Player`
  (`|AIMoveTo` self (0.0 0.0 0.0) (`GameplayStatics.GetPlayerCharacter` 0) 0.2
    (:`OnSuccess`
      (`KismetSystemLibrary.Delay` 0.2)
      (`self.Chase Player`))))

(fn `AddToReserve`
  (params (`Ammo Type` :type "/Game/TestAmmoEnum Enum" :default "NewEnumerator0") (Index :type Integer) (`Ammo To Add` :type Integer))
  (bind _ammotypes (`self.AmmoTypes`))
  (bind _returnvalue (select `/Game/TestAmmoEnum` `Ammo Type` :`NewEnumerator0` _ammotypes :`NewEnumerator1` _ammotypes :`NewEnumerator2` _ammotypes :`NewEnumerator3` _ammotypes :`NewEnumerator4` _ammotypes :`NewEnumerator5` _ammotypes :`NewEnumerator6` _ammotypes))
  (bind _output (`|GetArrayItem` _returnvalue Index))
  (bind (_ammotype _index _maxreserveammo _maxmagammo _reserveammo _loadedammo _has_) (break `/Game/AmmoInvStruct` _output))
  (bind _returnvalue_2 (+ `Ammo To Add` _reserveammo))
  (bind _returnvalue_3 (> _returnvalue_2 _maxreserveammo))
  (`KismetSystemLibrary.LogString` (`KismetStringLibrary.Conv_BoolToString` _returnvalue_3))
  (if _returnvalue_3
    (`KismetSystemLibrary.LogString` "Too Much Picked Up")
    (`self.Update Ammo Inventory And Push To HUD` _output _ammotype _index _maxreserveammo _maxmagammo _maxreserveammo _loadedammo _has_ Index _returnvalue)
    (else
      (`KismetSystemLibrary.LogString` "Adding Ammo")
      (`self.Update Ammo Inventory And Push To HUD` _output _ammotype _index _maxreserveammo _maxmagammo _returnvalue_2 _loadedammo _has_ Index _returnvalue))))

(fn `AmmoHud Test Method`
  (bind _asnew_hud (cast `/Game/Blueprints/NewHUD` (`PlayerController.GetHUD` (`GameplayStatics.GetPlayerController` 0)))
    (:`then`
      (bind (_reserveammo _loadedammo) (`self.GetAmmoForEquippedGun`))
      (`/Game/HUD_Widget.UpdateAmmoForWeaponSwap` (`/Game/Blueprints/NewHUD.HudRef` _asnew_hud) _reserveammo _loadedammo))
    (:`CastFailed`
      (`KismetSystemLibrary.LogString` "Hud Cast Failed"))))

(fn `Delete Currently Equipped`
  (bind _currentbpweapon (`self.CurrentBPWeapon`))
  ;[1 1 1] Delete the weapon object somehow
  (if (`KismetSystemLibrary.IsValid` _currentbpweapon)
    (`ActorComponent.K2_DestroyComponent` _currentbpweapon)
    (else
      (`KismetSystemLibrary.LogString` "Unable to delete"))))

(fn `Does Have Ammo Left in Mag`
  (returns (HasMoreThan0 :type Boolean))
  (bind (_reserveammo _loadedammo) (`self.GetAmmoForEquippedGun`))
  (if (< 0 _loadedammo)
    (`KismetSystemLibrary.LogString` "Has Ammo In Mag")
    (return true)
    (else
      (`KismetSystemLibrary.LogString` "Doesnt Has Ammo In Mag")
      (return false))))

(fn `Does Have Ammo Left in Reserve`
  (returns (HasMoreThan0 :type Boolean))
  (bind _reserveammo (`self.GetAmmoForEquippedGun`))
  (if (< 0 _reserveammo)
    (`KismetSystemLibrary.LogString` "Has Ammo In Mag" false)
    (return true)
    (else
      (`KismetSystemLibrary.LogString` "Doesnt Has Ammo In Mag" false)
      (return false))))

(fn `EquipWeapon`
  (params (WeaponIndex :type Integer))
  (bind _ammotypes (`self.AmmoTypes`))
  ;[1 1 1] Basic Equip weapon code that sets everything up on the backend
  (bind _output_get (set `self.CurrentEquippedWeapon` (`|GetArrayItem` (select `int` WeaponIndex :`0` _ammotypes :`1` _ammotypes :`2` _ammotypes :`3` _ammotypes :`4` _ammotypes :`5` _ammotypes) WeaponIndex)))
  (`KismetSystemLibrary.LogString` (`|GetEnumeratorNameAsString` (`.AmmoType_17_943C8CF5407E2593FC38ADBAA9B059CE` (break `/Game/AmmoInvStruct` _output_get)))))

(fn `GetAmmoForEquippedGun`
  (returns (ReserveAmmo :type Integer) (LoadedAmmo :type Integer) (Index :type Integer) (`Ammo Type` :type "/Game/TestAmmoEnum Enum"))
  (bind _ammotypes (`self.AmmoTypes`))
  (bind (_index _ammo_type) (`self.GetCurrentEquippedWeapon`))
  (bind (_ammotype _index_2 _maxreserveammo _maxmagammo _reserveammo _loadedammo) (break `/Game/AmmoInvStruct` (`|GetArrayItem` (select `/Game/TestAmmoEnum` _ammo_type :`NewEnumerator0` _ammotypes :`NewEnumerator1` _ammotypes :`NewEnumerator2` _ammotypes :`NewEnumerator3` _ammotypes :`NewEnumerator4` _ammotypes :`NewEnumerator5` _ammotypes :`NewEnumerator6` _ammotypes) _index)))
  (return _reserveammo _loadedammo _index _ammo_type))

(fn `GetCurrentEquippedWeapon`
  (returns (Index :type Integer) (`Ammo Type` :type "/Game/TestAmmoEnum Enum"))
  (bind (_ammotype _index) (break `/Game/AmmoInvStruct` (`self.CurrentEquippedWeapon`)))
  (return _index _ammotype))

(fn `GetPlayerControllerForWeapons`
  (returns (`AsBP First Person Player Controller` :type "/Game/FirstPerson/Blueprints/BP_FirstPersonPlayerController Object Reference"))
  (bind _asbp_first_person_player_controller (cast `/Game/FirstPerson/Blueprints/BP_FirstPersonPlayerController` (`GameplayStatics.GetPlayerController` 0)))
  (return _asbp_first_person_player_controller))

(fn `IsInteractable`
  (returns (Interactable :type Boolean))
  (return false))

(fn `IsInteractionObservable`
  (params (Target :type "Actor Object Reference"))
  (returns (IsObserveable :type Boolean)))

(fn `IsWeaponEquipped`
  (params (Index :type Integer))
  (returns (ReturnValue :type Boolean))
  (bind _index (`self.GetCurrentEquippedWeapon`))
  (return (== _index Index)))

(fn `Modify Player Armor`
  (params (`Damage Armor` :type Integer) (`Repair Armor` :type Integer) (BreakArmor :type Boolean))
  (bind _armor (`self.Armor`))
  (bind _returnvalue (+ _armor `Repair Armor`))
  (if BreakArmor
    (`KismetSystemLibrary.LogString` "Break Armor Completely")
    (elif (== `Repair Armor` 0)
      (bind _output_get (set `self.Armor` (- _armor `Damage Armor`)))
      (bind _asnew_hud (cast `/Game/Blueprints/NewHUD` (`PlayerController.GetHUD` (`GameplayStatics.GetPlayerController` 0))))
      (`/Game/HUD_Widget.UpdateArmorValue` (`/Game/Blueprints/NewHUD.HudRef` _asnew_hud) _output_get)
      (elif (> _returnvalue 3)
        (`KismetSystemLibrary.LogString` "Armor Is at max strength")
        (else
          (bind _output_get_2 (set `self.Armor` _returnvalue))
          (bind _asnew_hud_2 (cast `/Game/Blueprints/NewHUD` (`PlayerController.GetHUD` (`GameplayStatics.GetPlayerController` 0))))
          (`/Game/HUD_Widget.UpdateArmorValue` (`/Game/Blueprints/NewHUD.HudRef` _asnew_hud_2) _output_get_2))))))

(fn `Modify Player Health`
  (params (`Damage Amount` :type Integer) (`Heal Ammount` :type Integer) (`Kill Player` :type Boolean))
  (bind _health (`self.Health`))
  (bind _returnvalue (+ _health `Heal Ammount`))
  (if `Kill Player`
    (`KismetSystemLibrary.LogString` "Kill Player")
    (elif (== `Heal Ammount` 0)
      (bind _output_get (set `self.Health` (- _health `Damage Amount`)))
      (bind _asnew_hud (cast `/Game/Blueprints/NewHUD` (`PlayerController.GetHUD` (`GameplayStatics.GetPlayerController` 0))))
      (`/Game/HUD_Widget.UpdateHealthValue` (`/Game/Blueprints/NewHUD.HudRef` _asnew_hud) _output_get)
      (elif (> _returnvalue 3)
        (`KismetSystemLibrary.LogString` "Heal Health but too full")
        (else
          (bind _output_get_2 (set `self.Health` _returnvalue))
          (bind _asnew_hud_2 (cast `/Game/Blueprints/NewHUD` (`PlayerController.GetHUD` (`GameplayStatics.GetPlayerController` 0))))
          (`/Game/HUD_Widget.UpdateHealthValue` (`/Game/Blueprints/NewHUD.HudRef` _asnew_hud_2) _output_get_2))))))

(fn `ReloadCurrentWeapon`
  (bind _ammotypes (`self.AmmoTypes`))
  ;[1 1 1] Need to check if mag is full or not
  (bind _hasmorethan0 (`self.Does Have Ammo Left in Reserve`))
  (if _hasmorethan0
    (bind (_reserveammo _loadedammo _index _ammo_type) (`self.GetAmmoForEquippedGun`))
    (bind _returnvalue (select `/Game/TestAmmoEnum` _ammo_type :`NewEnumerator0` _ammotypes :`NewEnumerator1` _ammotypes :`NewEnumerator2` _ammotypes :`NewEnumerator3` _ammotypes :`NewEnumerator4` _ammotypes :`NewEnumerator5` _ammotypes :`NewEnumerator6` _ammotypes))
    (bind _output (`|GetArrayItem` _returnvalue _index))
    (bind (_ammotype _index_2 _maxreserveammo _maxmagammo _reserveammo_2 _loadedammo_2 _has_) (break `/Game/AmmoInvStruct` _output))
    (bind _returnvalue_2 (- _maxmagammo _loadedammo_2))
    (if (> _reserveammo_2 _returnvalue_2)
      (`self.Update Ammo Inventory And Push To HUD` _output _ammotype _index_2 _maxreserveammo _maxmagammo (- _reserveammo_2 _returnvalue_2) (+ _loadedammo_2 _returnvalue_2) _has_ _index _returnvalue)
      (else
        (`self.Update Ammo Inventory And Push To HUD` _output _ammotype _index_2 _maxreserveammo _maxmagammo 0 (+ _reserveammo_2 _loadedammo_2) _has_ _index _returnvalue)))
    (else
      (`KismetSystemLibrary.LogString` "Reserve Empty"))))

(fn `SetCurrentBP`
  (params (Weapon :type "/Game/FirstPerson/Blueprints/BP_Weapon_Component Object Reference"))
  (set `self.CurrentBPWeapon` Weapon))

(fn `Subtract MagAmmo`
  (bind _ammotypes (`self.AmmoTypes`))
  (bind (_reserveammo _loadedammo _index _ammo_type) (`self.GetAmmoForEquippedGun`))
  (bind _returnvalue (select `/Game/TestAmmoEnum` _ammo_type :`NewEnumerator0` _ammotypes :`NewEnumerator1` _ammotypes :`NewEnumerator2` _ammotypes :`NewEnumerator3` _ammotypes :`NewEnumerator4` _ammotypes :`NewEnumerator5` _ammotypes :`NewEnumerator6` _ammotypes))
  (bind _output (`|GetArrayItem` _returnvalue _index))
  (bind (_ammotype _index_2 _maxreserveammo _maxmagammo _reserveammo_2 _loadedammo_2 _has_) (break `/Game/AmmoInvStruct` _output))
  (bind _structout (setmembers `/Game/AmmoInvStruct` :`StructRef` _output :`Ammo Type` _ammotype :`Index` _index_2 :`MaxReserveAmmo` _maxreserveammo :`ReserveAmmo` _reserveammo_2 :`LoadedAmmo` (- _loadedammo_2 1) :`Has?` _has_))
  (`KismetArrayLibrary.Array_Set` _returnvalue _index _structout)
  (`KismetSystemLibrary.LogString` "Current Ammo: " false)
  (`KismetSystemLibrary.LogString` (`KismetStringLibrary.Conv_IntToString` _loadedammo_2) false))

(fn `SwapWeapon`
  (params (`Test Ammo Enum` :type "/Game/TestAmmoEnum Enum" :default "NewEnumerator0") (`Weapon INdex` :type Integer))
  (bind _asbp_first_person_player_controller (`self.GetPlayerControllerForWeapons`))
  (bind _has_ (`/Game/InventoryComponent.DoesPlayerHaveWeapon` (`/Game/FirstPerson/Blueprints/BP_FirstPersonPlayerController.Player Inventory` _asbp_first_person_player_controller) `Test Ammo Enum`))
  (if _has_
    ;[1 1 1] Check to see if BP component exists
    (if (`KismetSystemLibrary.IsValid` (`self.CurrentBPWeapon`))
      (bind _returnvalue (`self.IsWeaponEquipped` `Weapon INdex`))
      (if _returnvalue
        (`KismetSystemLibrary.LogString` "Weapon Already Equipped")
        (else
          (`self.Delete Currently Equipped`)
          (`KismetSystemLibrary.LogString` "Trying to Equip: ")
          (`KismetSystemLibrary.LogString` (`KismetStringLibrary.Conv_IntToString` `Weapon INdex`))
          (switch `/Game/TestAmmoEnum` `Test Ammo Enum`
            (:`NewEnumerator0`
              (`self.EquipWeapon` 0)
              (bind _returnvalue_2 (`AddComponent|NODE_AddBP_Weapon_Component-8`))
              (`self.SetCurrentBP` _returnvalue_2)
              (`self.AmmoHud Test Method`))
            (:`NewEnumerator1`
              (`self.EquipWeapon` 1)
              (bind _returnvalue_3 (`AddComponent|NODE_AddBP_Weapon_Component-11`))
              (`self.SetCurrentBP` _returnvalue_3)
              (`self.AmmoHud Test Method`))
            (:`NewEnumerator2`
              (bind _returnvalue_4 (`AddComponent|NODE_AddBP_Weapon_Component-16`))
              (`self.SetCurrentBP` _returnvalue_4))
            (:`NewEnumerator3`
              (bind _returnvalue_5 (`AddComponent|NODE_AddBP_Weapon_Component-17`))
              (`self.SetCurrentBP` _returnvalue_5))
            (:`NewEnumerator4`
              (bind _returnvalue_6 (`AddComponent|NODE_AddBP_Weapon_Component-18`))
              (`self.SetCurrentBP` _returnvalue_6))
            (:`NewEnumerator5`
              (bind _returnvalue_7 (`AddComponent|NODE_AddBP_Weapon_Component-19`))
              (`self.SetCurrentBP` _returnvalue_7)))))
      (else
        (`|ExecutionSequence`
          (:`then_0`
            (switch `/Game/TestAmmoEnum` `Test Ammo Enum`
              (:`NewEnumerator0`
                (`self.EquipWeapon` 0)
                (bind _returnvalue_8 (`AddComponent|NODE_AddBP_Weapon_Component-2`))
                (`self.SetCurrentBP` _returnvalue_8)
                (`self.AmmoHud Test Method`))
              (:`NewEnumerator1`
                (`self.EquipWeapon` 1)
                (bind _returnvalue_9 (`AddComponent|NODE_AddBP_Weapon_Component-9`))
                (`self.SetCurrentBP` _returnvalue_9)
                (`self.AmmoHud Test Method`))
              (:`NewEnumerator2`
                (bind _returnvalue_10 (`AddComponent|NODE_AddBP_Weapon_Component-12`))
                (`self.SetCurrentBP` _returnvalue_10))
              (:`NewEnumerator3`
                (bind _returnvalue_11 (`AddComponent|NODE_AddBP_Weapon_Component-13`))
                (`self.SetCurrentBP` _returnvalue_11))
              (:`NewEnumerator4`
                (bind _returnvalue_12 (`AddComponent|NODE_AddBP_Weapon_Component-14`))
                (`self.SetCurrentBP` _returnvalue_12))
              (:`NewEnumerator5`
                (bind _returnvalue_13 (`AddComponent|NODE_AddBP_Weapon_Component-15`))
                (`self.SetCurrentBP` _returnvalue_13)))))))
    (else
      (`KismetSystemLibrary.LogString` "DOESNT HAVE")
      (`KismetSystemLibrary.LogString` (`|GetEnumeratorNameAsString` `Test Ammo Enum`)))))

(fn `Update Ammo Inventory And Push To HUD`
  (params (StructRef :type "/Game/AmmoInvStruct Structure (by ref)") (`Ammo Type` :type "/Game/TestAmmoEnum Enum" :default "NewEnumerator0") (Index :type Integer) (MaxReserveAmmo :type Integer) (MaxMagAmmo :type Integer) (ReserveAmmo :type Integer) (LoadedAmmo :type Integer) (`Has?` :type Boolean) (Index1 :type Integer) (TargetArray :type "Array of /Game/AmmoInvStruct Structure (by ref)"))
  ;[1 1 1] This function is for Reloading mostly
  (bind _structout (setmembers `/Game/AmmoInvStruct` :`StructRef` StructRef :`Ammo Type` `Ammo Type` :`Index` Index :`MaxReserveAmmo` MaxReserveAmmo :`MaxMagAmmo` MaxMagAmmo :`ReserveAmmo` ReserveAmmo :`LoadedAmmo` LoadedAmmo :`Has?` `Has?`))
  (`KismetArrayLibrary.Array_Set` TargetArray Index1 _structout)
  ;;[1 1 1] Update the HUD
  (`self.AmmoHud Test Method`))

(fn `UserConstructionScript`)